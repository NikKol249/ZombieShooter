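; Player controller that shows the mouse cursor and drives where the player looks.
; On BeginPlay it adds the player movement Enhanced Input mapping context.
; Every tick it traces under the cursor on the Visibility channel and sends the hit location to the pawn through a LookAt message.
; The IA_Rotation input action separately sets the character's rotation from its X/Y value using a look-at rotation.
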(event `self.ReceiveBeginPlay`
  (bind _returnvalue (subsystem `EnhancedInputLocalPlayerSubsystem`))
  (set `self.bShowMouseCursor` true)
  (`/Engine/EditorBlueprintResources/StandardMacros.IsValid` _returnvalue
    (:`Is Valid`
      (`EnhancedInputSubsystemInterface.AddMappingContext` _returnvalue "/Game/Input/IMC_PlayerMovemen.IMC_PlayerMovemen" 0 (struct)))))

(event `self.ReceiveTick`
  (params (DeltaSeconds :type "Float (single-precision)"))
  (message `/Game/Blueprints/BPI_ZSCharacter.LookAt` (`GameplayStatics.GetPlayerPawn` 0) (`.Location` (`GameplayStatics.BreakHitResult` (`self.GetHitResultUnderCursorByChannel` "TraceTypeQuery1")))))

(event `EnhancedInput|/Game/Input/Actions/IA_Rotation`
  (params (ActionValue :type "Vector2D Structure") (ElapsedSeconds :type "Float (double-precision)") (TriggeredSeconds :type "Float (double-precision)") (InputAction :type "InputAction Object Reference" :default "/Game/Input/Actions/IA_Rotation.IA_Rotation"))
  (bind (_x _y) (`KismetMathLibrary.BreakVector2D` ActionValue))
  (:`Triggered`
    (`self.K2_SetActorRotation` (`GameplayStatics.GetPlayerCharacter` 0) (`KismetMathLibrary.FindLookAtRotation` (0.0 0.0 0.0) (`KismetMathLibrary.MakeVector` _x _y)) false)))

(fn `UserConstructionScript`)